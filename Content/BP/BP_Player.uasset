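; BP_Player represents a card-game player, owning heroes and four card zones: deck, hand, play and discard.
; Initialize stores deck data and applies a GAS setup effect; Setup spawns heroes and shuffled cards from data-table rows.
; MoveCardToZone handles transfers for drawing, refilling the hand to six and playing cards, with event calls announcing draws and plays.
; RefillDeckFromDiscard is an empty stub, so drawing from an empty deck prints an error.
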(fn `AddDefaultAbilities`
  (`AbilitySystemComponent.BP_ApplyGameplayEffectToSelf` :`self` (`self.GetAbilitySystemComponent`) :`GameplayEffectClass` "/Game/Data/GameEffects/GE_PlayerSetup.GE_PlayerSetup_C"))

(fn `DrawCard`
  (locals (bTryRefill :type Boolean))
  (set `local.bTryRefill` false)
  (if (`/Game/BP/BP_CardZone.IsEmpty` (`self.DeckZone`)) :!label _label
    (if (`local.bTryRefill`)
      (`KismetSystemLibrary.PrintString` "Error! No more cards!")
      (else
        (set `local.bTryRefill` true)
        (`self.RefillDeckFromDiscard`)
        (goto _label)))
    (else
      (bind _outcard (`/Game/BP/BP_CardZone.GetCardByIndex` (`self.DeckZone`) 0))
      (bind _outcard_2 (`self.MoveCardToZone` _outcard "NewEnumerator0"))
      (`self.ED_OnCardAction` _outcard_2 "NewEnumerator1"))))

(fn `GetZone`
  (params (ZoneType :type "/Game/Data/ECardZone Enum" :default "NewEnumerator4"))
  (returns (OutZone :type "/Game/BP/BP_CardZone Object Reference"))
  (switch `/Game/Data/ECardZone` ZoneType
    (:`NewEnumerator0`
      (return (`self.HandZone`)))
    (:`NewEnumerator1`
      (return (`self.DeckZone`)))
    (:`NewEnumerator2`
      (return (`self.PlayZone`)))
    (:`NewEnumerator3`
      (return (`self.DiscardZone`)))))

(fn `Initialize`
  (params (DeckData :type "/Game/Data/FDeckData Structure"))
  (set `self.DeckData` DeckData)
  (`self.AddDefaultAbilities`))

(fn `MoveCardToZone`
  (params (Card :type "/Game/BP/BP_Card Object Reference") (ToZone :type "/Game/Data/ECardZone Enum" :default "NewEnumerator4"))
  (returns (OutCard :type "/Game/BP/BP_Card Object Reference"))
  (bind _outzone (`self.GetZone` ToZone))
  (bind _outzone_2 (`self.GetZone` (`/Game/BP/BP_Card.CurrentZone` Card)))
  (`/Engine/EditorBlueprintResources/StandardMacros.IsValid` Card
    (:`Is Valid`
      (if (!= _outzone_2 _outzone)
        (`/Engine/EditorBlueprintResources/StandardMacros.IsValid` _outzone_2
          (:`Is Valid`
            (`/Game/BP/BP_CardZone.RemoveCard` _outzone_2 Card))
          (:`Is Not Valid`
            _))
        (bind _outcard (`/Game/BP/BP_CardZone.AddCard` _outzone Card))
        (set `/Game/BP/BP_Card.CurrentZone` ToZone _outcard)
        (return _outcard)))))

(fn `PlayCard`
  (params (CardToPlay :type "/Game/BP/BP_Card Object Reference"))
  (if (`/Game/BP/BP_Card.CanBePlayed` CardToPlay)
    (bind _outcard (`self.MoveCardToZone` CardToPlay "NewEnumerator2"))
    (`self.ED_OnCardAction` _outcard "NewEnumerator2")))

(fn `RefillDeckFromDiscard`)

(fn `RefillHand`
  (bind _returnvalue (- 6 (`/Game/BP/BP_CardZone.GetSize` (`self.HandZone`))))
  (if (> _returnvalue 0)
    (for _ (range (+ _returnvalue 1))
      (`self.DrawCard`))))

(fn `Setup`
  (`self.SetupHeroes`)
  (`self.SetupDeck`))

(fn `SetupDeck`
  (for _array_element (`.Cards_8_B65B84DB472B20FDE5E4EBB36CAC12B5` (break `/Game/Data/FDeckData` (`self.DeckData`)))
    (bind (_datatable _rowname) (break `DataTableRowHandle` _array_element))
    (bind _returnvalue (`|GetDataTableRow` _datatable _rowname)
      (:`then`
        (bind _returnvalue_2 (`|SpawnActorFromClass` "/Game/BP/BP_Card.BP_Card_C" (`self.GetTransform`) "Undefined" "OverrideRootScale" null null))
        (`/Game/BP/BP_Card.Initialize` _returnvalue_2 _returnvalue self)
        (`self.MoveCardToZone` _returnvalue_2 "NewEnumerator1"))))
  (`/Game/BP/BP_CardZone.Shuffle` (`self.DeckZone`)))

(fn `SetupHeroes`
  (for _array_element (`.Heroes_7_1E3BAAAA43BDA5F5B2ADC590AA9CD7E7` (break `/Game/Data/FDeckData` (`self.DeckData`)))
    (bind (_datatable _rowname) (break `DataTableRowHandle` _array_element))
    (bind _returnvalue (`|GetDataTableRow` _datatable _rowname)
      (:`then`
        (bind _returnvalue_2 (`|SpawnActorFromClass` "/Game/BP/BP_Hero.BP_Hero_C" (`self.GetTransform`) "Undefined" "OverrideRootScale" null null))
        (`/Game/BP/BP_Hero.Initialize` _returnvalue_2 _returnvalue self)
        (`KismetArrayLibrary.Array_Add` (`self.Heroes`) _returnvalue_2)
        (`self.ED_OnHeroSpawn` _returnvalue_2)))))

(fn `UserConstructionScript`
  (`|ExecutionSequence`
    (:`then_0`
      (bind _returnvalue (`|GenericCreateObject` "/Game/BP/BP_CardZone.BP_CardZone_C" self))
      (set `self.PlayZone` _returnvalue))
    (:`then_1`
      (bind _returnvalue_2 (`|GenericCreateObject` "/Game/BP/BP_CardZone.BP_CardZone_C" self))
      (set `self.DeckZone` _returnvalue_2))
    (:`then_2`
      (bind _returnvalue_3 (`|GenericCreateObject` "/Game/BP/BP_CardZone.BP_CardZone_C" self))
      (set `self.HandZone` _returnvalue_3))
    (:`then_3`
      (bind _returnvalue_4 (`|GenericCreateObject` "/Game/BP/BP_CardZone.BP_CardZone_C" self))
      (set `self.DiscardZone` _returnvalue_4))))