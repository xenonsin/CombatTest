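; BP_Card is a card actor Blueprint that holds one card's data and owner and reports whether it can be played.
; Initialize stores the data and owner passed in.
; CanBePlayed casts to Test1GameMode and allows play only during one specific CurrentPhase, returning false if the cast fails.
; GetValidTargets is an empty stub, and the event graph and construction script contain no logic.
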(fn `CanBePlayed`
  (returns (Result :type Boolean))
  (bind _astest_1game_mode (cast `/Game/Maps/CombatTest1/Test1GameMode` (`GameplayStatics.GetGameMode`))
    (:`then`
      (return (`|EnumEquality` (`/Game/Maps/CombatTest1/Test1GameMode.CurrentPhase` _astest_1game_mode) "NewEnumerator1")))
    (:`CastFailed`
      (return false))))

(fn `GetValidTargets`
  (params (TargetType :type "/Game/Data/ETargetType Enum" :default "NewEnumerator0"))
  (returns (OutActors :type "Array of Actor Object Reference"))
  (return))

(fn `Initialize`
  (params (Data :type "/Game/Data/FCardData Structure") (Owner :type "/Game/BP/BP_Player Object Reference"))
  (set `self.CardOwner` Owner)
  (set `self.Data` Data))

(fn `UserConstructionScript`)