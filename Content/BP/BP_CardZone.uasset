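; BP_CardZone is a container that holds an ordered array of cards for a card game.
; It exposes functions to add, remove by reference, fetch by index, shuffle, count and check for emptiness.
; Removal and index lookups guard against missing cards or invalid indices, and add and remove return the affected card.
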(fn `AddCard`
  (params (InCard :type "/Game/BP/BP_Card Object Reference"))
  (returns (OutCard :type "/Game/BP/BP_Card Object Reference"))
  (bind _returnvalue (`KismetArrayLibrary.Array_Add` (`self.Cards`) InCard))
  (return (`|GetArrayItem` (`self.Cards`) _returnvalue)))

(fn `GetCardByIndex`
  (params (Index :type Integer))
  (returns (OutCard :type "/Game/BP/BP_Card Object Reference"))
  (bind _cards (`self.Cards`))
  (if (`KismetArrayLibrary.Array_IsValidIndex` _cards Index)
    (return (`|GetArrayItem` _cards Index))
    (else
      (return null))))

(fn `GetSize`
  (returns (Size :type Integer))
  (return (`KismetArrayLibrary.Array_Length` (`self.Cards`))))

(fn `IsEmpty`
  (returns (Result :type Boolean))
  (return (<= (`KismetArrayLibrary.Array_Length` (`self.Cards`)) 0)))

(fn `RemoveCard`
  (params (CardToRemove :type "/Game/BP/BP_Card Object Reference"))
  (returns (OutCard :type "/Game/BP/BP_Card Object Reference"))
  (bind _returnvalue (`KismetArrayLibrary.Array_Find` (`self.Cards`) CardToRemove))
  (if (>= _returnvalue 0)
    (`KismetArrayLibrary.Array_Remove` (`self.Cards`) _returnvalue)
    (return CardToRemove)
    (else
      (return null))))

(fn `Shuffle`
  (`KismetArrayLibrary.Array_Shuffle` (`self.Cards`)))